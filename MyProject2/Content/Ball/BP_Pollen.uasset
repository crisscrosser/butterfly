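; BP_Pollen is a collectible pollen actor that awards a point when its sphere is hit.
; On any hit, it broadcasts OnBallTouched, plays a munch sound, increments Points on the player's third-person character and updates that character's HUD, then destroys itself.
; The hit handler does not check which actor struck the sphere, so the point always goes to player 0.
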(event OnComponentHit(Sphere)
  (params (HitComponent :type Primitive%20Component%20Object%20Reference) (OtherActor :type Actor%20Object%20Reference) (OtherComp :type Primitive%20Component%20Object%20Reference) (NormalImpulse :type Vector :default "0, 0, 0") (Hit :type Hit%20Result%20Structure%20%28by%20ref%29))
  (Utilities|FlowControl|Sequence
    (:then_0
      (Default|CallOnBallTouched))
    (:then_1
      (Audio|PlaySound2D "/Game/Audio/MUNCH.MUNCH" 1.0 1.0 0.0 0 0)
      (bind _asbp_third_person_character (Utilities|Casting|CastToBP_ThirdPersonCharacter (Game|GetPlayerCharacter 0)))
      (bind _output_get (Variables|/Game/ThirdPerson/Blueprints/BP_ThirdPersonCharacter.BP_ThirdPersonCharacter_C|SetPoints _asbp_third_person_character (+ (Variables|/Game/ThirdPerson/Blueprints/BP_ThirdPersonCharacter.BP_ThirdPersonCharacter_C|GetPoints _asbp_third_person_character) 1)))
      (Default|HUDUpdatePoints (Variables|/Game/ThirdPerson/Blueprints/BP_ThirdPersonCharacter.BP_ThirdPersonCharacter_C|GetHUD _asbp_third_person_character) _output_get)
      (Actor|DestroyActor))))

(event EventBeginPlay)

(event EventTick
  (params (DeltaSeconds :type Float%20%28single-precision%29)))

(fn ConstructionScript)