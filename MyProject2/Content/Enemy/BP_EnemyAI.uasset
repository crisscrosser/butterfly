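; Enemy AI pawn that chases the player on sight and damages them on contact.
; PawnSensing detection sets a seeing flag and starts an AIMoveTo toward the player character.
; Overlapping the third-person character subtracts health, updates its HUD, then destroys the enemy and asks the spawner found on BeginPlay to spawn near the character.
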(event OnSeePawn(PawnSensing)
  (params (Pawn :type Pawn%20Object%20Reference))
  (Variables|Default|SetisSeeingPlayer true)
  (CallFunction|FollowPlayer))

(event Custom|FollowPlayer
  (if (Variables|Default|GetisSeeingPlayer)
    (Development|PrintString "bro is cooked")
    (AI|AIMoveTo self "0, 0, 0" (Game|GetPlayerCharacter 0) 5.0 false)))

(event EventBeginPlay
  (bind _returnvalue (Actor|GetActorOfClass "/Game/Enemy/BP_EnemySpawner.BP_EnemySpawner_C"))
  (Variables|Default|SetEnemySpawner _returnvalue))

(event Collision|EventActorBeginOverlap
  (params (OtherActor :type Actor%20Object%20Reference))
  (bind _asbp_third_person_character (Utilities|Casting|CastToBP_ThirdPersonCharacter OtherActor))
  (Variables|/Game/ThirdPerson/Blueprints/BP_ThirdPersonCharacter.BP_ThirdPersonCharacter_C|SetHealth _asbp_third_person_character (- (Variables|/Game/ThirdPerson/Blueprints/BP_ThirdPersonCharacter.BP_ThirdPersonCharacter_C|GetHealth _asbp_third_person_character) 2e+01))
  (Default|SetHealth _asbp_third_person_character)
  (Default|HUDUpdateHealth (Variables|/Game/ThirdPerson/Blueprints/BP_ThirdPersonCharacter.BP_ThirdPersonCharacter_C|GetHUD _asbp_third_person_character) (Variables|/Game/ThirdPerson/Blueprints/BP_ThirdPersonCharacter.BP_ThirdPersonCharacter_C|GetHealth _asbp_third_person_character))
  (Actor|DestroyActor)
  (Default|SpawnNearCharacter (Variables|Default|GetEnemySpawner)))

(fn ConstructionScript)